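; BP_VSEnemyCharacter is an enemy character that damages the player on contact.
; When its capsule begins overlapping an actor tagged "Player", it looks up BP_Player with GetActorOfClass rather than using the overlapping actor, decrements Health and destroys the player at zero.
; Print strings trace each branch.
; UpdateWalkSpeed ignores its NewWalkSpeed input and sets a fixed max walk speed.
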(event OnComponentBeginOverlap(CapsuleComponent)
  (params (OverlappedComponent :type Primitive%20Component%20Object%20Reference) (OtherActor :type Actor%20Object%20Reference) (OtherComp :type Primitive%20Component%20Object%20Reference) (OtherBodyIndex :type Integer) (bFromSweep :type Boolean) (SweepResult :type Hit%20Result%20Structure%20%28by%20ref%29))
  (if (Actor|ActorHasTag OtherActor "Player")
    (Development|PrintString "PlayerHit")
    (bind _returnvalue (Actor|GetActorOfClass "/Game/Project/Player/BP_Player.BP_Player_C"))
    (if (> (Variables|/Game/Project/Player/BP_Player.BP_Player_C|GetHealth _returnvalue) 0)
      (bind _output_get (Variables|/Game/Project/Player/BP_Player.BP_Player_C|SetHealth _returnvalue (- (Variables|/Game/Project/Player/BP_Player.BP_Player_C|GetHealth _returnvalue) 1)))
      (if (<= _output_get 0)
        (Development|PrintString "Health0")
        (Actor|DestroyActor _returnvalue)
        (else
          (Development|PrintString "Health not 0")))
      (else
        (Development|PrintString "Health not 0 ijou")))
    (else
      (Development|PrintString "NotPlayerHit"))))

(event EventBeginPlay)

(event Collision|EventActorBeginOverlap
  (params (OtherActor :type Actor%20Object%20Reference)))

(fn ConstructionScript)

(fn UpdateWalkSpeed
  (params (NewWalkSpeed :type Float%20%28double-precision%29))
  (Variables|/Script/Engine.CharacterMovementComponent|SetMaxWalkSpeed (Variables|Character|GetCharacterMovement) 5e+02))