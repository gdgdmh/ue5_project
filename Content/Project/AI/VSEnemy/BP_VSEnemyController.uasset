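; BP_VSEnemyController is the AI controller for VS enemies, feeding the player's position to their behavior tree.
; On possess it runs BT_VSEnemy, and on BeginPlay it caches the BP_Player actor.
; Tick passes through a short Delay, throttling how often the player's location is written to the TargetLocation blackboard key, and prints an error if the player is invalid.
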(event EventBeginPlay
  (bind _returnvalue (Actor|GetActorOfClass "/Game/Project/Player/BP_Player.BP_Player_C"))
  (Variables|Default|SetPlayerActor _returnvalue))

(event EventTick
  (params (DeltaSeconds :type Float%20%28single-precision%29))
  ;[1 1 1] Set Player Location To Target Location
  (Utilities|FlowControl|Delay 0.2)
  (if (Utilities|IsValid (Variables|Default|GetPlayerActor))
    (bind _output_get (Variables|Default|SetTargetLocationVector (Transformation|GetActorLocation (Variables|Default|GetPlayerActor))))
    (AI|Components|Blackboard|SetValueasVector (Variables|Default|GetBlackboard) (Variables|Default|GetTargetLocation) _output_get)
    (else
      (Development|PrintString "Failed VSEnemyController Get Player Location"))))

(event EventPossess
  (params (PossessedPawn :type Pawn%20Object%20Reference))
  (AI|RunBehaviorTree "/Game/Project/AI/VSEnemy/BT_VSEnemy.BT_VSEnemy"))

(fn ConstructionScript)